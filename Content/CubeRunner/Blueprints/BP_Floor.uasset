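; BP_Floor is a floor segment for CubeRunner that fills itself with randomly spawned enemies.
; Its construction script builds a grid of arrow spawn points along each lane, shuffles them, and adds child actors through a weighted random branch.
; Player overlap with DestroyTrigger asks the game mode to extend the floor, while OutOfBound pauses the game and requests the end UI.
; GetAttachPoint exposes an arrow transform as the segment's attach point.
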(event `self.DestroyTrigger.OnComponentBeginOverlap`
  (params (OverlappedComponent :type "PrimitiveComponent Object Reference") (OtherActor :type "Actor Object Reference") (OtherComp :type "PrimitiveComponent Object Reference") (OtherBodyIndex :type Integer) (bFromSweep :type Boolean) (SweepResult :type "HitResult Structure (by ref)"))
  (if (== OtherActor (`GameplayStatics.GetPlayerCharacter` 0))
    (message `/Game/CubeRunner/Blueprints/BPI_BaseGame.CallExtendFloor` (`GameplayStatics.GetGameMode`))))

(event `self.OutOfBound.OnComponentBeginOverlap`
  (params (OverlappedComponent :type "PrimitiveComponent Object Reference") (OtherActor :type "Actor Object Reference") (OtherComp :type "PrimitiveComponent Object Reference") (OtherBodyIndex :type Integer) (bFromSweep :type Boolean) (SweepResult :type "HitResult Structure (by ref)"))
  (if (== (`GameplayStatics.GetPlayerCharacter` 0) OtherActor)
    (`GameplayStatics.SetGamePaused` true)
    (message `/Game/CubeRunner/Blueprints/BPI_BaseGame.CreateEndUI` (`GameplayStatics.GetGameMode`))))

(fn `GetAttachPoint`
  (returns (AttachPoint :type "Transform Structure"))
  (return (`SceneComponent.K2_GetComponentToWorld` (`self.Arrow`))))

(fn `InitEnemySpawnLocations`
  (for _array_element (`self.LanePositions`)
    (for _index (range 12)
      (bind _returnvalue (`AddComponent|NODE_AddArrowComponent-0` :`RelativeTransform` (`KismetMathLibrary.MakeTransform` (`KismetMathLibrary.MakeVector` (`KismetMathLibrary.Conv_IntToDouble` (* _index 400)) _array_element))))
      (`KismetArrayLibrary.Array_Add` (`self.SpawnLocations`) (`SceneComponent.K2_GetComponentToWorld` _returnvalue)))))

(fn `SpawnEnemy`
  (locals (RandomSpawnPoint :type "Array of Transform Structure"))
  (bind _output_get (set `local.RandomSpawnPoint` (`self.SpawnLocations`)))
  (`KismetArrayLibrary.Array_Shuffle` _output_get)
  (for _index (range 36)
    (switch `int` (`KismetMathLibrary.Conv_BoolToInt` (> (`KismetMathLibrary.RandomIntegerInRange` 1 10) 7))
      (:`0`
        (bind _returnvalue (`KismetMathLibrary.MakeRelativeTransform` (`|GetArrayItem` (`local.RandomSpawnPoint`) _index) (`self.GetTransform`)))
        (`AddComponent|NODE_AddChildActorComponent-1` :`RelativeTransform` _returnvalue))
      (:`1`
        (`AddComponent|NODE_AddChildActorComponent-2` :`RelativeTransform` _returnvalue)))))

(fn `UserConstructionScript`
  (`self.InitEnemySpawnLocations`)
  (`self.SpawnEnemy`))
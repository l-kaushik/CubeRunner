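; Game mode for CubeRunner that runs the endless floor, score, HUD and game-over screen.
; Floors chain through attach points, with the oldest destroyed on each extension.
; Score changes raise player speed past a rising threshold, or pause the game and show the end screen below zero.
; Each surviving score change resets a looping one-second inactivity timer, which spawns a death wall at the floor's end after about ten seconds.
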(event `self.ReceiveBeginPlay`
  (`self.initTiles`)
  (`self.initUI`)
  (`self.ActivityCounter`))

(event `AddScore`
  (params (Score :type Integer))
  (bind _returnvalue (`GameplayStatics.GetPlayerCharacter` 0))
  (bind _returnvalue_2 (+ Score (`self.CurrentScore`)))
  ;[0 0 0] Update player score according to the cube collied with
  (bind _output_get (set `self.CurrentScore` _returnvalue_2))
  (if (< _output_get 0)
    ;[0 0 0] Display End Screen
    (set `self.CurrentScore` 0)
    (`GameplayStatics.SetGamePaused` true)
    (`self.CreateEndScreenUI`)
    (message `/Game/CubeRunner/Blueprints/BPI_PlayerCharacter.SetDeltaLocationX` (`GameplayStatics.GetPlayerCharacter` 0) 0.0)
    (else
      (`/Game/CubeRunner/UI/WB_Hud.UpdateScore` (`self.UserInterface`) (`self.CurrentScore`))
      (if (> _returnvalue_2 (`self.ScoreThreshold`))
        ;[0 0 0] Increase player speed by 200 on every 10 poitns
        (bind _deltalocationx (message `/Game/CubeRunner/Blueprints/BPI_PlayerCharacter.GetDeltaLocationX` _returnvalue))
        (message `/Game/CubeRunner/Blueprints/BPI_PlayerCharacter.SetDeltaLocationX` _returnvalue (+ _deltalocationx 200.0))
        (set `self.ScoreThreshold` (+ (`self.ScoreThreshold`) 10))
        (`self.ActivityCounter`)
        (else
          (`self.ActivityCounter`))))))

(event `ActivityCounter`
  ;[0 0 0] If player not hitting any red or blue cube for certain amount of time then spawn a wall and kill
  (if (not (`self.isWallSpawned`))
    (bind _output_get (set `self.LastScoreUpdate` 0))
    (`/Game/CubeRunner/UI/WB_Hud.UpdateTime` (`self.UserInterface`) _output_get)
    (`KismetSystemLibrary.K2_SetTimerDelegate` (delegate `LastScoreCounter`) 1.0 true)))

(event `LastScoreCounter`
  (bind _lastscoreupdate (`self.LastScoreUpdate`))
  ;[0 0 0] If player not hitting any red or blue cube for certain amount of time then spawn a wall and kill
  (if (> (`self.LastScoreUpdate`) 10)
    (`self.SpawnWall`)
    (`/Game/CubeRunner/UI/WB_Hud.UpdateTime` (`self.UserInterface`) -1)
    (set `self.isWallSpawned` true)
    (else
      (`/Game/CubeRunner/UI/WB_Hud.UpdateTime` (`self.UserInterface`) _lastscoreupdate)
      (`/Engine/EditorBlueprintResources/StandardMacros.IncrementInt` _lastscoreupdate))))

(event `/Game/CubeRunner/Blueprints/BPI_BaseGame.SetScore`
  (params (Score :type Integer))
  (`self.AddScore` Score))

(event `/Game/CubeRunner/Blueprints/BPI_BaseGame.CallExtendFloor`
  (`self.ExtendFloor`))

(event `/Game/CubeRunner/Blueprints/BPI_BaseGame.CreateEndUI`
  (`self.CreateEndScreenUI`))

(fn `AddFloor`
  (bind _returnvalue (`|SpawnActorFromClass` "/Game/CubeRunner/Blueprints/BP_Floor.BP_Floor_C" (`self.FloorAttachPoint`) "Undefined" "MultiplyWithRoot" null null))
  (set `self.FloorAttachPoint` (`/Game/CubeRunner/Blueprints/BP_Floor.GetAttachPoint` _returnvalue))
  (`KismetArrayLibrary.Array_Add` (`self.Floors`) _returnvalue))

(fn `CreateEndScreenUI`
  (bind _returnvalue (`GameplayStatics.GetPlayerController` 0))
  (bind _returnvalue_2 (`|CreateWidget` "/Game/CubeRunner/UI/WB_EndScreen.WB_EndScreen_C"))
  (bind _output_get (set `self.EndScreen` _returnvalue_2))
  (`UserWidget.AddToViewport` _output_get 0)
  (`WidgetBlueprintLibrary.SetInputMode_UIOnlyEx` _returnvalue _returnvalue_2)
  (set `PlayerController.bShowMouseCursor` true _returnvalue))

(fn `ExtendFloor`
  (bind _floors (`self.Floors`))
  (bind _output (`|GetArrayItem` _floors))
  (`self.AddFloor`)
  (if (> (`KismetArrayLibrary.Array_Length` (`self.Floors`)) 2)
    (`self.K2_DestroyActor` _output)
    (`KismetArrayLibrary.Array_RemoveItem` _floors _output)))

(fn `initTiles`
  (for _ (range 3)
    (`self.AddFloor`)))

(fn `initUI`
  (bind _returnvalue (`|CreateWidget` "/Game/CubeRunner/UI/WB_Hud.WB_Hud_C"))
  (bind _output_get (set `self.UserInterface` _returnvalue))
  (`UserWidget.AddToViewport` _output_get 0)
  (`/Game/CubeRunner/UI/WB_Hud.UpdateScore` _output_get 0))

(fn `SpawnWall`
  (`|SpawnActorFromClass` "/Game/CubeRunner/Blueprints/BP_DeathWall.BP_DeathWall_C" (`self.FloorAttachPoint`) "Undefined" "MultiplyWithRoot" null null))

(fn `UserConstructionScript`)